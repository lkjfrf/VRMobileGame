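; VRPlayer is the player Blueprint for VR, with lateral movement and a brief attack state triggered by water.
; MoveRight input moves along the control rotation's yaw-only right vector.
; A Box overlap with a Water actor holds the Attack flag true for a short delay, then clears it.
; Tick draws a debug visibility trace forward from VRCamera, but its result is unused.
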(event `InputAxis|MoveRight` :overrideparent false
  (params (AxisValue :type "Float (single-precision)"))
  (`self.AddMovementInput` (`KismetMathLibrary.GetRightVector` (`KismetMathLibrary.MakeRotator` 0.0 0.0 (.yaw (`self.GetControlRotation`)))) AxisValue))

(event `self.ReceiveTick`
  (params (DeltaSeconds :type "Float (single-precision)"))
  (bind _vrcamera (`self.VRCamera`))
  (bind _returnvalue (`SceneComponent.K2_GetComponentLocation` _vrcamera))
  (`KismetSystemLibrary.LineTraceSingle` :`Start` _returnvalue :`End` (+ _returnvalue (* (`KismetMathLibrary.GetForwardVector` (`SceneComponent.K2_GetComponentRotation` _vrcamera)) 500.0)) :`TraceChannel` "TraceTypeQuery1" :`DrawDebugType` "ForOneFrame"))

(event `self.Box.OnComponentBeginOverlap`
  (params (OverlappedComponent :type "PrimitiveComponent Object Reference") (OtherActor :type "Actor Object Reference") (OtherComp :type "PrimitiveComponent Object Reference") (OtherBodyIndex :type Integer) (bFromSweep :type Boolean) (SweepResult :type "HitResult Structure (by ref)"))
  (cast `/Game/BluePrint/Water` OtherActor)
  (set `self.Attack` true)
  (`KismetSystemLibrary.Delay` 0.3)
  (set `self.Attack` false))

(fn `UserConstructionScript`)