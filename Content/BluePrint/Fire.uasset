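; Fire is a moving target actor that awards a point when a MobilePlayer or VRPlayer overlaps its Box.
; Tick moves it along world -X at constant speed, while a timeline drives a Time widget's progress and destroys it after a short delay.
; An overlap spawns a fire hit effect, briefly waits, destroys the actor and increments Score on either the mobile or VR game mode.
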(event `self.ReceiveBeginPlay`
  ;[1 1 1] 타이머 + 시간차 Destroy
  (bind _returnvalue (`|CreateWidget` "/Game/Widget/Time.Time_C"))
  (`WidgetComponent.SetWidget` (`self.Widget`) _returnvalue)
  (bind (_direction `_새_트랙_0`) (`Timeline|타임라인_0` :!via `PlayFromStart`)
    (:`Update`
      (`/Game/Widget/Time.SetProgress` _returnvalue `_새_트랙_0`))
    (:`Finished`
      (`KismetSystemLibrary.Delay` 3.0)
      (`self.K2_DestroyActor`))))

(event `self.ReceiveTick`
  (params (DeltaSeconds :type "Float (single-precision)"))
  ;[1 1 1] 8.0뒤에 노래스폰해야 맞음
  (`self.K2_AddActorWorldOffset` (* (-1.0 0.0 0.0) (* DeltaSeconds 1200.0))))

(event `self.Box.OnComponentBeginOverlap`
  (params (OverlappedComponent :type "PrimitiveComponent Object Reference") (OtherActor :type "Actor Object Reference") (OtherComp :type "PrimitiveComponent Object Reference") (OtherBodyIndex :type Integer) (bFromSweep :type Boolean) (SweepResult :type "HitResult Structure (by ref)"))
  (bind _returnvalue (`GameplayStatics.GetGameMode`))
  ;[1 1 1] Hit
  (cast `/Game/BluePrint/MobilePlayer` OtherActor
    (:`then`
      _)
    (:`CastFailed`
      (cast `/Game/BluePrint/VRPlayer` OtherActor)))
  (`GameplayStatics.SpawnEmitterAtLocation` "/Game/AdvancedMagicFX12/Particles/P_ky_hit_fire.P_ky_hit_fire" (`SceneComponent.K2_GetComponentLocation` (`self.FX`)))
  (`KismetSystemLibrary.Delay` 0.2)
  (`self.K2_DestroyActor`)
  (bind _asgame_mode_mobile (cast `/Game/BluePrint/GameModeMobile` _returnvalue)
    (:`then`
      (set `/Game/BluePrint/GameModeMobile.Score` (+ (`/Game/BluePrint/GameModeMobile.Score` _asgame_mode_mobile) 1) _asgame_mode_mobile))
    (:`CastFailed`
      (bind _asgame_mode_vr (cast `/Game/BluePrint/GamemodeVR` _returnvalue))
      (set `/Game/BluePrint/GamemodeVR.Score` (+ (`/Game/BluePrint/GamemodeVR.Score` _asgame_mode_vr) 1) _asgame_mode_vr))))

(fn `UserConstructionScript`)